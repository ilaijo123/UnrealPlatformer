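; NewAi_BP is a simple 2D patrolling AI that drops a PickUp_Bp when a BP_projectile hits its box.
; Tick moves it along world X; when nearly stopped, a FlipFlop alternately negates or keeps Movement and toggles the facing flag.
; Sprite facing mirrors via X scale from velocity, using the flag at zero.
; A separate UpdateAnimation event selects the flipbook by speed.
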(event OnComponentBeginOverlap(Box)
  (params (OverlappedComponent :type Primitive%20Component%20Object%20Reference) (OtherActor :type Actor%20Object%20Reference) (OtherComp :type Primitive%20Component%20Object%20Reference) (OtherBodyIndex :type Integer) (bFromSweep :type Boolean) (SweepResult :type Hit%20Result%20Structure%20%28by%20ref%29))
  (Utilities|Casting|CastToBP_projectile OtherActor)
  (Rendering|SetVisibility (Variables|Default|GetSprite) false false)
  (Utilities|FlowControl|Delay 0.1)
  (Game|SpawnActorfromClass "/Game/blueprts/PickUp_Bp.PickUp_Bp_C" (Transformation|GetActorTransform) "Undefined" "MultiplyWithRoot" 0 0)
  (Actor|DestroyActor))

(event Custom|UpdateAnimation
  ;[1 1 1] Handle Animation
  (Sprite|SetFlipbook (Variables|Default|GetSprite) (select (> (Math|Vector|VectorLength (Transformation|GetVelocity)) 0.0) 0 0)))

(event EventTick
  (params (DeltaSeconds :type Float%20%28single-precision%29))
  ;[1 1 1] Tick - Updates animation
  (Utilities|FlowControl|Sequence
    (:then_0
      (Pawn|Input|AddMovementInput "1.000000, 0, 0" (Variables|Default|GetMovement) false)
      (if (< (Math|Vector|VectorLength (Transformation|GetVelocity)) 1.0)
        (Utilities|FlowControl|FlipFlop
          (:A
            (Variables|Default|SetMovement (* (Variables|Default|GetMovement) -1.0))
            (Variables|Default|SetbisMovingRight false))
          (:B
            (Variables|Default|SetMovement (* (Variables|Default|GetMovement) 1.0))
            (Variables|Default|SetbisMovingRight true)))))
    (:then_1
      (Math|Float|CompareFloat (.X (Math|Vector|BreakVector (Variables|/Script/Engine.MovementComponent|GetVelocity (Pawn|GetMovementComponent)))) 0.0
        (:>
          (Transformation|SetWorldScale3D (Variables|Default|GetSprite) "0.100000,0.100000,0.100000" :!label _label))
        (:==
          (if (Variables|Default|GetbisMovingRight)
            (goto _label)
            (else
              (Transformation|SetWorldScale3D (Variables|Default|GetSprite) "-0.100000,0.100000,0.100000" :!label _label_2))))
        (:<
          (goto _label_2))))))

(event EventBeginPlay
  (Class|ActorComponent|SetIsReplicated (Variables|Default|GetSprite) true))

(fn ConstructionScript)